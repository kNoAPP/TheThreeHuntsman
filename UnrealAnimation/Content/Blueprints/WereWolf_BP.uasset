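; WereWolf_BP is a werewolf Blueprint that demonstrates blood splatter with decals left where the particles land.
; A left mouse press spawns the blood emitter at the skeletal mesh's spine socket and binds its particle collision event.
; Each collision creates a dynamic decal material with a random Frame value for variety, then places a randomly sized, temporary stain aligned to the hit normal.
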(event Custom|OnCollideEvent
  (params (EventName :type Name) (EmitterTime :type Float%20%28single-precision%29) (ParticleTime :type Integer) (Location :type Vector) (Velocity :type Vector) (Direction :type Vector) (Normal :type Vector) (BoneName :type Name) (PhysMat :type Physical%20Material%20Object%20Reference))
  (bind _returnvalue (Rendering|Material|CreateDynamicMaterialInstance "/Game/VFX/Materials/M_BloodColourStain_Decal.M_BloodColourStain_Decal" "None" "None" :!class /Script/Engine.KismetMaterialLibrary))
  (Rendering|Material|SetScalarParameterValue _returnvalue "Frame" (Math|Conversions|ToFloat(Integer) (Math|Random|RandomInteger 11)) :!class /Script/Engine.MaterialInstanceDynamic)
  (Rendering|Decal|SpawnDecalatLocation _returnvalue (Math|Conversions|ToVector(Float) (Math|Random|RandomFloatinRange 2e+01 5e+01)) Location (Math|Conversions|RotationFromXVector Normal) 2e+01))

(event EventBeginPlay)

(event Collision|EventActorBeginOverlap
  (params (OtherActor :type Actor%20Object%20Reference)))

(event EventTick
  (params (DeltaSeconds :type Float%20%28single-precision%29)))

(event Input|MouseEvents|LeftMouseButton
  (params (Key :type Key%20Structure :default "None"))
  (:Pressed
    (bind _returnvalue (Effects|SpawnEmitteratLocation "/Game/VFX/ParticleSystem/P_bloodSplat.P_bloodSplat" (Transformation|GetSocketLocation (Variables|Default|GetSkeletalMesh) "CATRigSpine1")))
    (EventDispatchers|BindEventtoOnParticleCollide _returnvalue (delegate Custom|OnCollideEvent))))

(fn ConstructionScript)